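; Player controller for editing voxel worlds at runtime with sphere, box and projection brushes, plus a key that launches asteroids at the cursor.
; Tick traces under the mouse and updates the active tool's marker, while HUD and held keys select add, remove, flatten or paint.
; Sphere and box edit per click; projection repeats on a timer while held.
; Successful projection sculpts and flattens make the foliage manager swap nearby instances for actors.
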(event Custom|ProjectionEditEvent
  (bind _mode (CallFunction|GetMode))
  (bind _radius (CallFunction|GetProjectionRadius))
  (bind _ui (Variables|Default|GetUI))
  (bind _currenthitposition (Variables|CurrentVariables|GetCurrentHitPosition))
  (bind _currenthitposition_2 (Variables|CurrentVariables|GetCurrentHitPosition))
  (bind _widget (Default|GetWidget _ui))
  (bind _wbp_voxelhud (Variables|/Voxel/WBP_VoxelUI.WBP_VoxelUI_C|GetWBP_VoxelHUD _ui))
  (bind _debug (Default|IsDebugging _widget))
  (bind __ (Default|GetStrength _wbp_voxelhud))
  ;[1 1 1] Projection edit
  (Utilities|IsValid (Variables|CurrentVariables|GetCurrentVoxelWorld)
    (:Is%20Valid
      (if (and (Game|Player|IsInputKeyDown "LeftMouseButton") (Utilities|Enum|Equal(Enum) (CallFunction|GetTool) "Projection"))
        (switch Utilities|FlowControl|Switch|SwitchonEVoxelMode _mode
          (:Add
            (bind (_failreason _lockername) (Class|VoxelProjectionTools|SetValueProjectionAsync (Variables|CurrentVariables|GetCurrentVoxelWorld) _currenthitposition (Variables|CurrentVariables|GetCurrentHitNormal) _radius (Utilities|Select :Index _mode :Add (* __ -1.0) :Remove __ :Flatten 0.0 :Paint 0.0) 0 2e+02 4e+02 0.5 0.0001 _debug :!label _label)
              (:Success
                (if true
                  (CallFunction|AfterWorldEdit _radius _currenthitposition)))
              (:Failed
                (Development|PrintString (Utilities|String|Append "SetValueProjection: " (Utilities|String|EnumtoString _failreason) " " _lockername) false))))
          (:Remove
            (goto _label))
          (:Flatten
            (bind _returnvalue (Class|VoxelTools|Flatten (Variables|CurrentVariables|GetCurrentVoxelWorld) (Variables|CurrentVariables|GetCurrentHitPosition) (Variables|Default|GetFlattenNormal) _radius 0.1 false false false 0.0001 _debug))
            (if _returnvalue
              (CallFunction|AfterWorldEdit _radius _currenthitposition_2)))
          (:Paint
            (bind (_failreason_2 _lockername_2) (Class|VoxelProjectionTools|SetMaterialProjectionAsync (Variables|CurrentVariables|GetCurrentVoxelWorld) _currenthitposition_2 (Variables|CurrentVariables|GetCurrentHitNormal) (CallFunction|GetPaintMaterial) 0 _radius 2e+02 4e+02 0.5 0.0001 _debug)
              (:Failed
                (Development|PrintString (Utilities|String|Append "SetMaterialProjection: " (Utilities|String|EnumtoString _failreason_2) " " _lockername_2) false)))))))))

(event Custom|After%20World%20Edit
  (params (Rad :type Float%20%28single-precision%29) (Loc :type Vector))
  (Utilities|FlowControl|Delay 0.02)
  (bind _foliagemanager (Variables|Default|GetFoliageManager)
    (:then
      (Class|InceptionFoliage|SwapInstancewithActor _foliagemanager Loc (* Rad 4.0) (Utilities|Array|MakeArray "ObjectTypeQuery1" "ObjectTypeQuery2")))
    (:else)))

(event EventBeginPlay
  ;[0.5847 1 0.2889] BeginPlay
  (Variables|Default|SetbShowMouseCursor true)
  (Utilities|Time|SetTimerbyEvent (delegate Custom|ProjectionEditEvent) (Variables|Parameters|GetEditDelay) true)
  ;;[1 1 1] Spawn UI
  (bind _returnvalue (UserInterface|CreateWidget "/Voxel/WBP_VoxelUI.WBP_VoxelUI_C" self))
  (bind _output_get (Variables|Default|SetUI _returnvalue))
  (UserInterface|Viewport|AddtoViewport _output_get 0)
  ;;[1 1 1] Spawn markers
  (bind _returnvalue_2 (Game|SpawnActorfromClass "/Script/Voxel.VoxelSphereMarker" (Math|Transform|MakeTransform "0, 0, 0") "Undefined" 0 (Game|Player|GetPlayerPawn 0)))
  (Variables|Markers|SetSphere%20Marker _returnvalue_2)
  (bind _returnvalue_3 (Game|SpawnActorfromClass "/Script/Voxel.VoxelProjectionMarker" (Math|Transform|MakeTransform "0, 0, 0") "Undefined" 0 (Game|Player|GetPlayerPawn 0)))
  (Variables|Markers|SetProjection%20Marker _returnvalue_3)
  (bind _returnvalue_4 (Game|SpawnActorfromClass "/Script/Voxel.VoxelBoxMarker" (Math|Transform|MakeTransform "0, 0, 0") "Undefined" 0 (Game|Player|GetPlayerPawn 0)))
  (Variables|Markers|SetBox%20Marker _returnvalue_4)
  (Rendering|SetActorHiddenInGame (Variables|Markers|GetProjection%20Marker) true)
  (Rendering|SetActorHiddenInGame (Variables|Markers|GetSphere%20Marker) true)
  (Rendering|SetActorHiddenInGame (Variables|Markers|GetBox%20Marker) true)
  (bind _outactors (Actor|GetAllActorsOfClass "/Game/Inception/Blueprints/Foliage/BP_FoliageManager.BP_FoliageManager_C"))
  (Variables|Default|SetFoliageManager (Utilities|Array|Get(acopy) _outactors)))

(event EventTick
  (params (DeltaSeconds :type Float%20%28single-precision%29))
  (bind (_locationx _locationy) (Game|Player|GetMousePosition))
  (bind _self self)
  (bind _projection_marker (Variables|Markers|GetProjection%20Marker))
  (bind _sphere_marker (Variables|Markers|GetSphere%20Marker))
  (bind _box_marker (Variables|Markers|GetBox%20Marker))
  (bind _returnvalue (Math|Vector2D|MakeVector2D _locationx _locationy))
  (bind (_worldposition _worlddirection) (Class|GameplayStatics|DeprojectScreentoWorld _self _returnvalue))
  ;[0.2389 0.6141 1] Tick
  (if (Pawn|IsLocalPlayerController)
    ;;[1 1 1] Linetrace
    (bind _outhit (Collision|LineTraceByChannel _worldposition (+ _worldposition (* _worlddirection 1e+06)) "TraceTypeQuery1" false 0 "None"))
    (bind _asvoxel_world (Utilities|Casting|CastToVoxelWorld (.HitActor (Collision|BreakHitResult _outhit))))
    (Variables|CurrentVariables|SetCurrentVoxelWorld _asvoxel_world)
    (Variables|CurrentVariables|SetCurrentHitPosition (.ImpactPoint (Collision|BreakHitResult _outhit)))
    (Variables|CurrentVariables|SetCurrentHitNormal (.Normal (Collision|BreakHitResult _outhit)))
    ;;[1 1 1] Set markers
    (Rendering|SetActorHiddenInGame (Variables|Markers|GetProjection%20Marker) true)
    (Rendering|SetActorHiddenInGame (Variables|Markers|GetSphere%20Marker) true)
    (Rendering|SetActorHiddenInGame (Variables|Markers|GetBox%20Marker) true)
    (switch Utilities|FlowControl|Switch|SwitchonEVoxelTool (CallFunction|GetTool)
      (:Projection
        (Rendering|SetActorHiddenInGame _projection_marker false)
        (Class|VoxelProjectionMarker|UpdateProjectionMarker _projection_marker (Variables|CurrentVariables|GetCurrentVoxelWorld) (CallFunction|GetMode) (Variables|CurrentVariables|GetCurrentHitPosition) (Variables|CurrentVariables|GetCurrentHitNormal) (CallFunction|GetProjectionRadius) 4e+02 2e+02))
      (:Sphere
        (Rendering|SetActorHiddenInGame _sphere_marker false)
        (Class|VoxelSphereMarker|UpdateSphereMarker _sphere_marker (Variables|CurrentVariables|GetCurrentVoxelWorld) (CallFunction|GetMode) (Class|VoxelWorld|GlobaltoLocal (Variables|CurrentVariables|GetCurrentVoxelWorld) (Variables|CurrentVariables|GetCurrentHitPosition)) (Variables|Default|GetRadius)))
      (:Box
        (Rendering|SetActorHiddenInGame _box_marker false)
        (Class|VoxelBoxMarker|UpdateBoxMarker _box_marker (Variables|CurrentVariables|GetCurrentVoxelWorld) (CallFunction|GetMode) (Class|VoxelBlueprintLibrary|MakeBoxfromGlobalPositionandRadius (Variables|CurrentVariables|GetCurrentVoxelWorld) (Variables|CurrentVariables|GetCurrentHitPosition) (Variables|Default|GetRadius)))))))

(event Input|MouseEvents|MouseWheelAxis
  (params (AxisValue :type Float%20%28single-precision%29))
  ;[1 1 1] Radius change
  (Variables|Default|SetRadius (Math|Float|Max(Float) (+ (* AxisValue (Variables|Parameters|GetRadiusChangeSpeed)) (Variables|Default|GetRadius)) 0.0)))

(event Input|KeyboardEvents|Backspace
  (params (Key :type Key%20Structure :default "None"))
  (bind _returnvalue (Math|Random|RandomUnitVectorinConeinDegrees "1.000000,1.000000,1.000000" 1.0))
  ;[1 1 1] Asteroid spawn
  (:Pressed
    (bind _returnvalue_2 (Game|SpawnActorfromClass "/Voxel/Example/VoxelAsteroid/VoxelAsteroid.VoxelAsteroid_C" (Math|Transform|MakeTransform (+ (Variables|CurrentVariables|GetCurrentHitPosition) (* _returnvalue 1e+05)) "0, 0, 0" (Math|Conversions|ToVector(Float) (Math|Random|RandomFloatinRange 1.0 25.0))) "Undefined" 0 0))
    (Physics|SetPhysicsLinearVelocity (Variables|/Voxel/Example/VoxelAsteroid/VoxelAsteroid.VoxelAsteroid_C|GetStaticMesh _returnvalue_2) (* _returnvalue -5e+04) false "None")))

(event Input|KeyboardEvents|H
  (params (Key :type Key%20Structure :default "None"))
  (bind _ui (Variables|Default|GetUI))
  ;[1 1 1] Hide UI
  (:Pressed
    (switch Utilities|FlowControl|Switch|SwitchonESlateVisibility (Widget|GetVisibility _ui)
      (:Visible
        (Widget|SetVisibility _ui "Hidden" :!label _label))
      (:Hidden
        (Widget|SetVisibility _ui "Visible"))
      (:SelfHitTestInvisible
        (goto _label)))))

(event Input|MouseEvents|LeftMouseButton
  (params (Key :type Key%20Structure :default "None"))
  (bind _radius (Variables|Default|GetRadius))
  (bind _currentvoxelworld (Variables|CurrentVariables|GetCurrentVoxelWorld))
  (bind _radius_2 (Variables|Default|GetRadius))
  (bind _currentvoxelworld_2 (Variables|CurrentVariables|GetCurrentVoxelWorld))
  (bind _currenthitposition (Variables|CurrentVariables|GetCurrentHitPosition))
  (bind _currentvoxelworld_3 (Variables|CurrentVariables|GetCurrentVoxelWorld))
  (bind _currenthitposition_2 (Variables|CurrentVariables|GetCurrentHitPosition))
  (bind _currentvoxelworld_4 (Variables|CurrentVariables|GetCurrentVoxelWorld))
  (bind _returnvalue (Class|VoxelBlueprintLibrary|MakeBoxfromGlobalPositionandRadius _currentvoxelworld_3 _currenthitposition _radius_2))
  (bind _returnvalue_2 (Class|VoxelWorld|GlobaltoLocal _currentvoxelworld_2 _currenthitposition_2))
  ;[1 1 1] Sphere/Box edit
  (:Pressed
    (Utilities|IsValid (Variables|CurrentVariables|GetCurrentVoxelWorld)
      (:Is%20Valid
        (switch Utilities|FlowControl|Switch|SwitchonEVoxelTool (CallFunction|GetTool)
          (:Sphere
            (switch Utilities|FlowControl|Switch|SwitchonEVoxelMode (CallFunction|GetMode)
              (:Add
                (Class|VoxelSphereTools|AddSphere _currentvoxelworld_4 _returnvalue_2 _radius))
              (:Remove
                (bind _returnvalue_3 (Class|VoxelSphereTools|RemoveSphere _currentvoxelworld_4 _returnvalue_2 _radius))
                (if _returnvalue_3
                  _))
              (:Paint
                (Class|VoxelSphereTools|SetMaterialSphere _currentvoxelworld_4 _returnvalue_2 _radius (CallFunction|GetPaintMaterial) 0))))
          (:Box
            (switch Utilities|FlowControl|Switch|SwitchonEVoxelMode (CallFunction|GetMode)
              (:Add
                (Class|VoxelBoxTools|AddBox _currentvoxelworld _returnvalue))
              (:Remove
                (Class|VoxelBoxTools|RemoveBox _currentvoxelworld _returnvalue))
              (:Paint
                (Class|VoxelBoxTools|SetMaterialBox _currentvoxelworld _returnvalue (CallFunction|GetPaintMaterial))))))))))

(event Input|MouseEvents|LeftMouseButton
  (params (Key :type Key%20Structure :default "None"))
  ;[1 1 1] Flatten cached normal
  (:Pressed
    (Variables|Default|SetFlattenNormal (Variables|CurrentVariables|GetCurrentHitNormal))))

(fn ConstructionScript)

(fn GetMode
  (if (Default|IsPainting (Default|GetWidget (Variables|Default|GetUI)))
    (return "Paint")
    (elif (Game|Player|IsInputKeyDown (Variables|Parameters|GetFlattenKey))
      (return "Flatten")
      (elif (Game|Player|IsInputKeyDown (Variables|Parameters|GetAddKey))
        (return "Add")
        (else
          (return "Remove"))))))

(fn GetPaintMaterial
  (return (Default|GetPaintMaterial (Default|GetWidget (Variables|Default|GetUI)))))

(fn GetTool
  (bind _tool (Default|GetTool (Variables|/Voxel/WBP_VoxelUI.WBP_VoxelUI_C|GetWBP_VoxelHUD (Variables|Default|GetUI))))
  (return _tool))

(fn GetProjectionRadius
  (bind _radius (Variables|Default|GetRadius))
  (bind _currentvoxelworld (Variables|CurrentVariables|GetCurrentVoxelWorld))
  (if (Utilities|IsValid _currentvoxelworld)
    (return (* _radius (Variables|/Script/Voxel.VoxelWorld|GetVoxelSize _currentvoxelworld) 0.1))
    (else
      (return (* _radius 1e+01)))))